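; BP_Projectile is a projectile actor that deals damage on sphere overlap and then destroys itself.
; An overlapped actor carrying AttackedTag receives a one-time TakeDamageMessage with the Damage value, so the tag selects whether Player or Enemy is the target.
; A second sequence branch prints a debug string and destroys the projectile when the overlapped actor's Instigator is not a controlled pawn.
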(event `self.Sphere.OnComponentBeginOverlap`
  (params (OverlappedComponent :type "PrimitiveComponent Object Reference") (OtherActor :type "Actor Object Reference") (OtherComp :type "PrimitiveComponent Object Reference") (OtherBodyIndex :type Integer) (bFromSweep :type Boolean) (SweepResult :type "HitResult Structure (by ref)"))
  (`|ExecutionSequence`
    (:`then_0`
      ;[1 1 1] Deal damage if contact is made with target Player or Enemy
      (if (`self.ActorHasTag` OtherActor (`self.AttackedTag`))
        (`/Engine/EditorBlueprintResources/StandardMacros.DoOnce` false
          (:`Completed`
            (message `/Game/SystemDesign/BP_Interface_Enemy.Take Damage` OtherActor (`self.Damage`))
            (`self.K2_DestroyActor`)))))
    (:`then_1`
      ;[1 1 1] Delete bullet if contact is made with a non-target pawn
      (if (not (`Pawn.IsPawnControlled` (`Actor.Instigator` OtherActor)))
        (`KismetSystemLibrary.PrintString` "Bye")
        (`self.K2_DestroyActor`)))))

(fn `UserConstructionScript`)