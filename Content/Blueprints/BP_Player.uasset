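; Player character Blueprint that adds a HUD and handles a second special attack.
; BeginPlay creates the HUD widget, and every Tick pushes the health ratio to it.
; Special Attack 2 launches the character upward, plays a two-handed montage, then briefly slows global time after a short delay.
; An unwired Camera Glide graph holds a timeline-lerped toggle between follow and perspective cameras, but never runs.
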(event `self.ReceiveBeginPlay`
  (`parent.ReceiveBeginPlay`)
  (bind _returnvalue (`|CreateWidget` "/Game/Blueprints/UserInterface/HUD_Widget.HUD_Widget_C" (`GameplayStatics.GetPlayerController` 0)))
  (bind _output_get (set `self.HUD Widget` _returnvalue))
  (`UserWidget.AddToViewport` _output_get 0))

(event `self.ReceiveTick`
  (params (DeltaSeconds :type "Float (single-precision)"))
  (`parent.ReceiveTick` DeltaSeconds)
  (`self.UpdateStats`))

(event `self.UpdateStats`
  (`self.UpdateHealth` (`self.HUD Widget`) (/ (`self.HealthPoints`) (`self.HealthPoints Max`))))

(event `InputAction|Special Attack 2`
  (params (Key :type "Key Structure"))
  (bind _charactermovement (`self.CharacterMovement`))
  (:`Pressed`
    (`CharacterMovementComponent.AddImpulse` _charactermovement (0.0 0.0 800.0) true)
    (`CharacterMovementComponent.AddForce` _charactermovement (0.0 0.0 800.0))
    (`self.PlayAnimMontage` "/Game/Animations/Frank_RPG_2Handed/Animations/2Hand_SpecialAttack2.2Hand_SpecialAttack2")
    (`KismetSystemLibrary.Delay` 0.37)
    (`GameplayStatics.SetGlobalTimeDilation` 0.4)
    (`KismetSystemLibrary.Delay` 2.0)
    (`GameplayStatics.SetGlobalTimeDilation` 1.0)))

(fn `UserConstructionScript`
  (`parent.UserConstructionScript`))