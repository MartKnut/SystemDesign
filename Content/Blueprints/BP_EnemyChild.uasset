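; Melee enemy character that attacks, blocks, takes hits and dies, driven by events for each action.
; Attack and block events play montages, while CheckHit tests the sword socket's distance to the nearest target and triggers effects and an OnHit message.
; Received hits either play a block reaction or subtract fixed health, with backward impulses and death ending in destruction.
; Unblocked hits use brief global time dilation as hit-stop.
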(event Collision|EventActorBeginOverlap
  (params (OtherActor :type Actor%20Object%20Reference))
  (|CallParentFunction OtherActor) ; This node is disabled and will not be called.\nDrag off pins to build functionality.
)

(event EventCheckHit
  (|CheckForHitEnemy))

(event EventOnHit
  (params (Actor :type Actor%20Object%20Reference))
  (|CallsOnHitonEnemy Actor))

(event EventTick
  (params (DeltaSeconds :type Float%20%28single-precision%29))
  (|CallParentFunction DeltaSeconds) ; This node is disabled and will not be called.\nDrag off pins to build functionality.
)

(event EventSetDetected
  (params (Detected :type Boolean))
  (Variables|Default|SetDetected Detected))

(event EventBeginPlay
  (|CallParentFunction) ; This node is disabled and will not be called.\nDrag off pins to build functionality.
)

(event EventEnemyAttack)

(event EventEnemyLightAttack
  (|LightAttackCombo_2))

(event EventEnemyHeavyAttack
  (|HeavyAttackCombo_2))

(event EventEnemyBlocking
  (|BlockingAction_2))

(fn ConstructionScript
  (|CallParentFunction))

(fn GetDetected
  (return (Variables|Default|GetDetected)))

(fn GetLockedOnto
  (return 0))