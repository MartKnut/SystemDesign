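; AI controller for the Frost Wraith enemy, handling its behavior tree, patrol setup and target detection.
; On BeginPlay it runs BehaviorTree_FrostWraith and copies the BP_AnotherEnemy pawn's patrol-loop flag to the Blackboard.
; Perception uses interface party checks, then updates "Seen" and the pawn's detection and lock-on, skipping the last stored enemy.
; GetLockedOnto returns the target; other interface functions return stub values.
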(event `self.ReceiveBeginPlay`
  ;[1 1 1] Runs Behaviour Tree and Pathing
  (set `self.Pawn1` (`self.K2_GetPawn`))
  (`self.RunBehaviorTree` "/Game/Blueprints/NEW_AI/BehaviorTree_FrostWraith.BehaviorTree_FrostWraith")
  (bind _asbp_another_enemy (cast `/Game/Blueprints/BP_AnotherEnemy` (`self.K2_GetPawn`)))
  (bind _output_get (set `self.MyPawn` _asbp_another_enemy))
  (`BlackboardComponent.SetValueAsBool` (`AIBlueprintHelperLibrary.GetBlackboard` null) "PathLooping" (`/Game/Blueprints/NPC_AI(Old)/PatrolPath.IsLooping` (`/Game/Blueprints/BP_AnotherEnemy.PatrolPath` _output_get))))

(event `self.AIPerception.OnTargetPerceptionUpdated`
  (params (Actor :type "Actor Object Reference") (Stimulus :type "AIStimulus Structure"))
  (bind _returnvalue (`self.K2_GetPawn`))
  ;[1 1 1] Detects Player
  (bind _party_number (message `/Game/Blueprints/BPInterface_CharacterACTIONS.GetParty` _returnvalue))
  (bind _true_ (message `/Game/Blueprints/BPInterface_CharacterACTIONS.IsAnEnemy` Actor _party_number))
  (if (and _true_ (!= Actor (`self.Enemy`)))
    (bind _output_get (set `self.LockedOnto` Actor))
    (`BlackboardComponent.SetValueAsBool` (`AIBlueprintHelperLibrary.GetBlackboard` null) "Seen" Stimulus_bSuccessfullySensed)
    (message `/Game/Blueprints/BPInterface_Enemy.SetDetected` _returnvalue Stimulus_bSuccessfullySensed)
    (set `self.Enemy` Actor)
    (message `/Game/Blueprints/BPInterface_CharacterACTIONS.LockOn` _returnvalue Stimulus_bSuccessfullySensed _output_get)))

(fn `Blocking`
  (returns (Blocking :type Boolean))
  (return false))

(fn `GetDetected`
  (returns (Detected :type Boolean))
  (return false))

(fn `GetLockedOnto`
  (returns (LockedOnto :type "Actor Object Reference"))
  (return (`self.LockedOnto`)))

(fn `GetParty`
  (returns (`Party Number` :type Integer))
  (return 0))

(fn `IsAnEnemy`
  (params (Party :type Integer))
  (returns (`True?` :type Boolean))
  (return false))

(fn `UserConstructionScript`)